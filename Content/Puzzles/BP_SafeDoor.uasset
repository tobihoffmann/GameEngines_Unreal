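; Puzzle safe door that swings open and closed when its OpenSafeDoor and CloseSafeDoor events are called.
; BeginPlay caches the static mesh's world rotation as the closed pose.
; A timeline drives a yaw offset, combined with that cached rotation so the swing is relative to the door's placed orientation.
; Closing reverses the same timeline.
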(event Custom|OpenSafeDoor
  ;[1 1 1] Open and Close Safe Door
  (bind _zaxis (Timeline|Timeline_0 Play)
    (:Update
      (Transformation|SetWorldRotation (Variables|Debug|GetStaticMeshComponent) (Math|Rotator|CombineRotators (Math|Rotator|MakeRotator 0.0 0.0 _zaxis) (Variables|Default|GetDefaultRotation)) false false))))

(event Custom|CloseSafeDoor
  ;[1 1 1] Open and Close Safe Door
  (bind _zaxis (Timeline|Timeline_0 Reverse)
    (:Update
      (Transformation|SetWorldRotation (Variables|Debug|GetStaticMeshComponent) (Math|Rotator|CombineRotators (Math|Rotator|MakeRotator 0.0 0.0 _zaxis) (Variables|Default|GetDefaultRotation)) false false))))

(event EventBeginPlay
  ;[1 1 1] Open and Close Safe Door
  (Variables|Default|SetDefaultRotation (Transformation|GetWorldRotation (Variables|Debug|GetStaticMeshComponent))))

(fn ConstructionScript)