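; BP_Building_Door2 is an interactable building door that can require an inventory item to unlock.
; On BeginPlay it stores its starting rotation and unlocks itself if the required item ID is zero.
; Interacting while locked searches the first-person character's inventory for that ID and only unlocks the door.
; Later interactions toggle it, playing or reversing a timeline that adds yaw to the starting rotation.
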(event EventBeginPlay
  (Variables|Default|SetDefaultRotation (Transformation|GetWorldRotation (Variables|Default|GetSM_Building_Door2)))
  (if (== 0 (Variables|Default|GetNecessaryItemID))
    (Variables|Default|SetIsLocked false)))

(event EventInteract
  (params (Interactor :type Actor%20Object%20Reference))
  (if (Variables|Default|GetIsLocked)
    (bind _asfirst_person_character (Utilities|Casting|CastToFirstPersonCharacter Interactor))
    (for _array_element (Variables|/Game/FirstPersonBP/InventorySystem/InventoryComponent.InventoryComponent_C|GetInventory (Variables|/Game/FirstPersonBP/Blueprints/FirstPersonCharacter.FirstPersonCharacter_C|GetInventoryComponent _asfirst_person_character))
      (if (== (.Item_ID (Utilities|Struct|BreakItemStructure (Utilities|Struct|BreakSlotStructure _array_element))) (Variables|Default|GetNecessaryItemID))
        (Variables|Default|SetIsLocked false)))
    (elif (Variables|Default|GetIsOpen)
      (Variables|Default|SetIsOpen false)
      (bind _zaxis (Timeline|Timeline_1 Reverse)
        (:Update
          (Transformation|SetWorldRotation (Variables|Default|GetSM_Building_Door2) (Math|Rotator|CombineRotators (Math|Rotator|MakeRotator 0.0 0.0 _zaxis) (Variables|Default|GetDefaultRotation)) false false)))
      (else
        (Variables|Default|SetIsOpen true)
        (Timeline|Timeline_1 Play)))))

(fn ConstructionScript)